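; BP_Health is a health pickup that heals the player character when something overlaps its Box.
; On BeginPlay it caches player 0's BP_ThirdPersonCharacter.
; Any overlap, without checking the overlapping actor, adds HealingAmount to that character's CurrentHealth, clamped to MaxHealth.
; It then calls the character's CastToUpdateHealth, plays a confirmation sound and destroys itself.
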(event OnComponentBeginOverlap(Box)
  (params (OverlappedComponent :type Primitive%20Component%20Object%20Reference) (OtherActor :type Actor%20Object%20Reference) (OtherComp :type Primitive%20Component%20Object%20Reference) (OtherBodyIndex :type Integer) (bFromSweep :type Boolean) (SweepResult :type Hit%20Result%20Structure%20%28by%20ref%29))
  (bind _character (Variables|Default|GetCharacter))
  (Variables|/Game/GameModes/ThirdPerson/Blueprints/BP_ThirdPersonCharacter.BP_ThirdPersonCharacter_C|SetCurrentHealth _character (Math|Float|Clamp(Float) (+ (Variables|/Game/GameModes/ThirdPerson/Blueprints/BP_ThirdPersonCharacter.BP_ThirdPersonCharacter_C|GetCurrentHealth _character) (Variables|Default|GetHealingAmount)) 0.0 (Variables|/Game/GameModes/ThirdPerson/Blueprints/BP_ThirdPersonCharacter.BP_ThirdPersonCharacter_C|GetMaxHealth _character)))
  (Default|CasttoUpdateHealth _character)
  (Audio|PlaySound2D "/Game/Sounds/Pickup/abs-confirm-1.abs-confirm-1" 1.0 1.0 0.0 0 0)
  (Actor|DestroyActor))

(event EventBeginPlay
  (bind _asbp_third_person_character (Utilities|Casting|CastToBP_ThirdPersonCharacter (Game|GetPlayerCharacter 0)))
  (Variables|Default|SetCharacter _asbp_third_person_character))

(fn ConstructionScript)