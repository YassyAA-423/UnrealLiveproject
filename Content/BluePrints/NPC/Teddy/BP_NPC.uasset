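; Teddy NPC that gives the player a quest to collect a lost loved one's notes and reacts to their progress.
; Overlapping its Box with BP_ThirdPersonCharacter checks NoteCount to pick the request, a progress question, or a farewell thanks once enough notes are held.
; CastToWidget, despite its name, creates a new WBP_Mission each time, whose instruction text shows the line on screen until a timed Delay removes it.
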(event OnComponentBeginOverlap(Box)
  (params (OverlappedComponent :type Primitive%20Component%20Object%20Reference) (OtherActor :type Actor%20Object%20Reference) (OtherComp :type Primitive%20Component%20Object%20Reference) (OtherBodyIndex :type Integer) (bFromSweep :type Boolean) (SweepResult :type Hit%20Result%20Structure%20%28by%20ref%29))
  (bind _asbp_third_person_character (Utilities|Casting|CastToBP_ThirdPersonCharacter OtherActor))
  (if (>= (Variables|/Game/GameModes/ThirdPerson/Blueprints/BP_ThirdPersonCharacter.BP_ThirdPersonCharacter_C|GetNoteCount _asbp_third_person_character) 5)
    (bind (_returnvalue _textblock_dialoguetext) (CallFunction|CasttoWidget))
    (Variables|/Script/UMG.TextBlock|SetText _textblock_dialoguetext "Thanks… I haven't the heart to read these till now… I miss her…. Good Luck Out There…")
    (UserInterface|Viewport|AddtoViewport _returnvalue 0)
    (Utilities|FlowControl|Delay 5.0)
    (Widget|RemovefromParent _returnvalue)
    (elif (<= (Variables|/Game/GameModes/ThirdPerson/Blueprints/BP_ThirdPersonCharacter.BP_ThirdPersonCharacter_C|GetNoteCount _asbp_third_person_character) 0)
      (bind (_returnvalue_2 _textblock_dialoguetext_2) (CallFunction|CasttoWidget))
      (Variables|/Script/UMG.TextBlock|SetText _textblock_dialoguetext_2 "Hey… I know you can't stay here any longer.. Do you think you can do me one last favor? Can you grab her Notes? I figure they can keep me company…                         (Press F to collect the Notes)")
      (UserInterface|Viewport|AddtoViewport _returnvalue_2 0)
      (Utilities|FlowControl|Delay 7.0)
      (Widget|RemovefromParent _returnvalue_2)
      (else
        (bind (_returnvalue_3 _textblock_dialoguetext_3) (CallFunction|CasttoWidget))
        (Variables|/Script/UMG.TextBlock|SetText _textblock_dialoguetext_3 "Did you find them? ")
        (UserInterface|Viewport|AddtoViewport _returnvalue_3 0)
        (Utilities|FlowControl|Delay 3.0)
        (Widget|RemovefromParent _returnvalue_3)))))

(fn ConstructionScript)

(fn CasttoWidget
  (bind _returnvalue (UserInterface|CreateWidget "/Game/UI/Pickups/NPC/WBP_Mission.WBP_Mission_C"))
  (bind _output_get (Variables|Default|SetActiveDialogue _returnvalue))
  (return _returnvalue (Variables|/Game/UI/Pickups/NPC/WBP_Mission.WBP_Mission_C|GetTextBlock_Intructions _output_get)))