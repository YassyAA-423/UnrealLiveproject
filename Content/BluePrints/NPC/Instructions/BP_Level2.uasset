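; BP_Level2 is a one-shot trigger that shows a level 2 hint about finding keys for the locked window to escape.
; When BP_ThirdPersonCharacter overlaps its Box, it creates WBP_Level2, sets the hint text and adds it to the viewport.
; After a timed delay it removes the widget and destroys itself.
; A CastToWidget function creates a WBP_Mission widget, but the overlap logic does not call it.
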(event OnComponentBeginOverlap(Box)
  (params (OverlappedComponent :type Primitive%20Component%20Object%20Reference) (OtherActor :type Actor%20Object%20Reference) (OtherComp :type Primitive%20Component%20Object%20Reference) (OtherBodyIndex :type Integer) (bFromSweep :type Boolean) (SweepResult :type Hit%20Result%20Structure%20%28by%20ref%29))
  (Utilities|Casting|CastToBP_ThirdPersonCharacter OtherActor)
  (bind _returnvalue (UserInterface|CreateWidget "/Game/UI/Pickups/NPC/WBP_Level2.WBP_Level2_C"))
  (bind _output_get (Variables|Default|SetActiveInstructions _returnvalue))
  (Variables|/Script/UMG.TextBlock|SetText (Variables|/Game/UI/Pickups/NPC/WBP_Level2.WBP_Level2_C|GetTextBlock_DialogueText _output_get) "The Window is Down the hall. I'm Pretty sure there's a lock on it. I better finds the keys. Then I can finally leave this place...")
  (UserInterface|Viewport|AddtoViewport _returnvalue 0)
  (Utilities|FlowControl|Delay 7.0)
  (Widget|RemovefromParent _returnvalue)
  (Actor|DestroyActor))

(fn ConstructionScript)

(fn CasttoWidget
  (bind _returnvalue (UserInterface|CreateWidget "/Game/UI/Pickups/NPC/WBP_Mission.WBP_Mission_C"))
  (bind _output_get (Variables|Default|SetActiveDialogue _returnvalue))
  (return _returnvalue (Variables|/Game/UI/Pickups/NPC/WBP_Mission.WBP_Mission_C|GetTextBlock_Intructions _output_get)))