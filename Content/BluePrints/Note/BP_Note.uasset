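; BP_Note is a collectible note that the player picks up with the IA_Pickup input while inside its Box.
; Box overlap with BP_ThirdPersonCharacter toggles the actor's input, so the pickup responds only at close range.
; Pickup decrements the game mode's Remaining count, shows a Testing widget and increments the character's NoteCount.
; It then plays a 2D sound and destroys the note.
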(event OnComponentEndOverlap(Box)
  (params (OverlappedComponent :type Primitive%20Component%20Object%20Reference) (OtherActor :type Actor%20Object%20Reference) (OtherComp :type Primitive%20Component%20Object%20Reference) (OtherBodyIndex :type Integer))
  (Utilities|Casting|CastToBP_ThirdPersonCharacter OtherActor)
  (Input|DisableInput (Game|GetPlayerController 0)))

(event OnComponentBeginOverlap(Box)
  (params (OverlappedComponent :type Primitive%20Component%20Object%20Reference) (OtherActor :type Actor%20Object%20Reference) (OtherComp :type Primitive%20Component%20Object%20Reference) (OtherBodyIndex :type Integer) (bFromSweep :type Boolean) (SweepResult :type Hit%20Result%20Structure%20%28by%20ref%29))
  (Utilities|Casting|CastToBP_ThirdPersonCharacter OtherActor)
  (Input|EnableInput (Game|GetPlayerController 0)))

(event Input|EnhancedActionEvents|EnhancedInputActionIA_Pickup
  (params (ActionValue :type Boolean) (ElapsedSeconds :type Float%20%28double-precision%29) (TriggeredSeconds :type Float%20%28double-precision%29) (InputAction :type Input%20Action%20Object%20Reference :default "/Game/GameModes/ThirdPerson/Input/Actions/IA_Pickup.IA_Pickup"))
  (:Started
    (bind _asbp_third_person_game_mode (Utilities|Casting|CastToBP_ThirdPersonGameMode (Game|GetGameMode)))
    (bind _result (Math|Integer|DecrementInt (Variables|/Game/GameModes/ThirdPerson/Blueprints/BP_ThirdPersonGameMode.BP_ThirdPersonGameMode_C|GetRemaining _asbp_third_person_game_mode))
      (:%20%20
        (Variables|/Game/GameModes/ThirdPerson/Blueprints/BP_ThirdPersonGameMode.BP_ThirdPersonGameMode_C|SetRemaining _asbp_third_person_game_mode _result)
        (bind _returnvalue (UserInterface|CreateWidget "/Game/UI/OverlayWidgets/Testing.Testing_C"))
        (UserInterface|Viewport|AddtoViewport _returnvalue 0)
        (bind _asbp_third_person_character (Utilities|Casting|CastToBP_ThirdPersonCharacter (Game|GetPlayerCharacter 0)))
        (Variables|/Game/GameModes/ThirdPerson/Blueprints/BP_ThirdPersonCharacter.BP_ThirdPersonCharacter_C|SetNoteCount _asbp_third_person_character (+ (Variables|/Game/GameModes/ThirdPerson/Blueprints/BP_ThirdPersonCharacter.BP_ThirdPersonCharacter_C|GetNoteCount _asbp_third_person_character) 1))
        (Audio|PlaySound2D "/Game/Sounds/Pickup/abs-popup-3.abs-popup-3" 1.0 1.0 0.0 0 0)
        (Actor|DestroyActor)))))

(fn ConstructionScript)